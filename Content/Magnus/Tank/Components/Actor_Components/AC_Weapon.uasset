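; Tank weapon actor component that fires projectiles from the turret cannon's Muzzle socket, gated by a firing delay.
; Fire spawns a BP_Projectile within a spread cone, makes cannon and projectile ignore each other, plays sound, camera shake and particles, then returns whether it fired.
; Separate events eject a physics-impulsed casing at the Breach socket and set cannon recoil offset.
; AddHUD is an empty stub.
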(event `Start Delay`
  (`KismetSystemLibrary.Delay` (`self.Firing Delay`))
  (set `self.Can Fire` true))

(event `Eject Shell`
  (bind _returnvalue (`|SpawnActorFromClass` (`self.Casing`) (`SceneComponent.GetSocketTransform` (`/Game/Parents/BP_Turret.Cannon` (`self.Turret`)) "Breach" "RTS_World") "Undefined" "MultiplyWithRoot" null null))
  (`PrimitiveComponent.AddImpulse` (`Actor.GetComponentByClass` _returnvalue "/Script/Engine.StaticMeshComponent") (`self.Ejection Impulse`) "None" false))

(event `Recoil Cannon`
  (params (Recoil :type "Float (double-precision)"))
  (`SceneComponent.K2_SetRelativeLocation` (`/Game/Parents/BP_Turret.Cannon` (`self.Turret`)) (`KismetMathLibrary.MakeVector` Recoil) false false))

(fn `Add HUD`
  (params (Controller :type "PlayerController Object Reference"))
  (returns (Widget :type "Widget Object Reference"))
  (return null))

(fn `Fire`
  (returns (Return :type Boolean))
  (bind _cannon (`/Game/Parents/BP_Turret.Cannon` (`self.Turret`)))
  (bind (_returnvalue_location _returnvalue_rotation _returnvalue_scale) (`KismetMathLibrary.BreakTransform` (`SceneComponent.GetSocketTransform` _cannon "Muzzle" "RTS_World")))
  (bind _returnvalue (`KismetMathLibrary.MakeRotFromX` (`KismetMathLibrary.RandomUnitVectorInConeInDegrees` (`SceneComponent.GetForwardVector` _cannon) (`self.Spread`))))
  (if (`self.Can Fire`)
    (set `self.Can Fire` false)
    (bind _returnvalue_2 (`|SpawnActorFromClass` "/Game/Magnus/Projectile/BP_Projectile.BP_Projectile_C" (`KismetMathLibrary.MakeTransform` _returnvalue_location _returnvalue _returnvalue_scale) "AlwaysSpawn" "MultiplyWithRoot" null (`self.Impact Damage`) (`self.Muzzle Velocity`) (`self.Projectile Radius`) (`/Game/Parents/BP_Turret.Tank` (`self.Turret`))))
    (`PrimitiveComponent.IgnoreActorWhenMoving` (`/Game/Parents/BP_Turret.Cannon` (`self.Turret`)) _returnvalue_2 true)
    (`PrimitiveComponent.IgnoreActorWhenMoving` (`Actor.GetComponentByClass` _returnvalue_2 "/Script/Engine.SphereComponent") (`self.GetOwner` (`/Game/Parents/BP_Turret.Cannon` (`self.Turret`))) true)
    (`GameplayStatics.PlaySoundAtLocation` null _returnvalue_location (struct) 1.0 1.0 0.0 null null null null)
    (`GameplayStatics.PlayWorldCameraShake` (`self.Cam Shake`) _returnvalue_location 0.0 3000.0)
    (`NiagaraFunctionLibrary.SpawnSystemAtLocation` (`self.Particles`) _returnvalue_location _returnvalue)
    (`self.Start Delay`)
    (return true)
    (else
      (return false))))