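; BP_Minigun is a tank turret minigun that must spin up before firing and is blocked from starting while overheated.
; Construction creates a dynamic heat material and passes it, with the spinning mesh and projectile settings, to an overheat weapon component set as the turret's weapon.
; Fire plays a timeline that drives the component's spin-up and calls parent Fire on forward completion.
; Release calls the parent and reverses the timeline to spin down.
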(event `self.Fire`
  (if (not (`/Game/Magnus/Tank/Components/Actor_Components/AC_Overheat_Weapon.Overheated` (`self.Overheat Weapon`)))
    (bind (_direction _spin) (`Timeline|MG Timeline` :!label _label)
      (:`Update`
        (`/Game/Magnus/Tank/Components/Actor_Components/AC_Overheat_Weapon.Spin Up` (`self.Overheat Weapon`) _spin))
      (:`Finished`
        (if (`|EnumEquality` _direction "Forward")
          (`parent.Fire`))))))

(event `self.Release`
  (`parent.Release`)
  (goto _label :!via `Reverse`))

(fn `UserConstructionScript`
  (`parent.UserConstructionScript`)
  (bind _returnvalue (`PrimitiveComponent.CreateDynamicMaterialInstance` (`self.Minigun`) 1 "/Game/Magnus/Tank/Material_Instances/MI_Minigun.MI_Minigun" "None"))
  (bind _returnvalue_2 (`AddComponent|NODE_AddAC_Overheat_Weapon-3` :`Heat Material` _returnvalue :`Overheat Delay` 4.0 :`Spinner` (`self.Minigun`) :`Cooldown Delay` 0.8 :`Turret` self :`Projectile Class` "/Game/Magnus/Projectile/BP_Proj_Mag_MG.BP_Proj_Mag_MG_C" :`Spread` 1.0 :`Firing Delay` 0.1 :`Casing` null :`Particles` null :`Cam Shake` null))
  (bind _output_get (set `self.Overheat Weapon` _returnvalue_2))
  (set `self.Weapon` _output_get))