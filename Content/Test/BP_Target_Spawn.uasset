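; Test spawner actor that keeps a BP_Magnus target tank with a BP_Standard turret at its own transform.
; On BeginPlay it spawns the tank, stores it, prints its name and calls IsTarget on it.
; Tick starts a one-second delayed respawn when the tank is invalid.
; The Spawning flag also satisfies that condition, so only the pending Delay absorbs repeat triggers.
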(event `self.ReceiveBeginPlay`
  (`self.Spawn`))

(event `Spawn`
  (bind _returnvalue (`|SpawnActorFromClass` "/Game/Magnus/Tank/BP_Magnus.BP_Magnus_C" (`self.GetTransform`) "Undefined" "MultiplyWithRoot" null "/Game/Magnus/Tank/Turrets/BP_Standard.BP_Standard_C" null))
  (bind _output_get (set `self.Tank` _returnvalue))
  (`KismetSystemLibrary.PrintString` (`KismetSystemLibrary.GetDisplayName` _output_get) true true (struct :`G` 0.049684 :`B` 1.0 :`A` 1.0))
  (`/Game/Parents/BP_Tank.Is Target` _output_get))

(event `self.ReceiveTick`
  (params (DeltaSeconds :type "Float (single-precision)"))
  (if (not (and (`KismetSystemLibrary.IsValid` (`self.Tank`)) (not (`self.Spawning`))))
    (set `self.Spawning` true)
    (`KismetSystemLibrary.Delay` 1.0)
    (`self.Spawn`)
    (set `self.Spawning` false)))

(fn `UserConstructionScript`)