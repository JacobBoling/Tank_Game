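; Standard turret Blueprint for the Magnus tank that fires a limited-ammo projectile weapon.
; The construction script calls its parent, then adds an ammo weapon component configured with projectile, ammo capacity, firing delay, shell casing, particles and camera shake.
; On a successful fire, a recoil timeline drives the cannon's kickback and an event track on it triggers shell ejection.
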(event `self.Fire`
  (bind _return (`/Game/Magnus/Tank/Components/Actor_Components/AC_Weapon.Fire` (`self.Weapon`)))
  (if _return
    (bind (_direction _recoil) (`Timeline|Recoil Timeline` :!via `PlayFromStart`)
      (:`Update`
        (`/Game/Magnus/Tank/Components/Actor_Components/AC_Weapon.Recoil Cannon` (`self.Weapon`) _recoil))
      (:`Eject`
        (`/Game/Magnus/Tank/Components/Actor_Components/AC_Weapon.Eject Shell` (`self.Weapon`))))))

(fn `UserConstructionScript`
  (`parent.UserConstructionScript`)
  (bind _returnvalue (`AddComponent|NODE_AddAC_Ammo_Weapon-0` :`Max Ammo` 25 :`Turret` self :`Projectile Class` "/Game/Magnus/Projectile/BP_Proj_Mag_Std.BP_Proj_Mag_Std_C" :`Firing Delay` 1.0 :`Casing` "/Game/Magnus/Casing/BP_Casing.BP_Casing_C" :`Ejection Impulse` (-80.0 0.0 1000.0) :`Particles` "/Game/Magnus/Tank/Components/Particles/FXS_Firing_Particles.FXS_Firing_Particles" :`Cam Shake` "/Game/Magnus/Tank/Components/Cam_Shake/AC_Cam_Shake.AC_Cam_Shake_C"))
  (bind _output_get (set `self.Ammo Weapon` _returnvalue))
  (set `self.Weapon` _output_get))