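; Parent tank turret that snaps onto a socket on the tank's hull and forwards fire, release and HUD setup to its weapon.
; Rotator and Elevator components handle clamped yaw and pitch, set absolutely or stepped by scope input.
; Artillery turrets turn the whole tank for scope rotation and ignore direct orientation updates.
; A muzzle line trace returns the aim impact point; its hit-indicator code is disconnected.
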(event `Fire`
  (`/Game/Magnus/Tank/Components/Actor_Components/AC_Weapon.Fire` (`self.Weapon`)))

(event `Release`
  (`/Game/Magnus/Tank/Components/Actor_Components/AC_Weapon.Release` (`self.Weapon`)))

(event `self.Set Tank`
  (params (Tank :type "/Game/Parents/BP_Tank Object Reference"))
  (`parent.Set Tank` Tank)
  (`self.K2_AttachToComponent` (`/Game/Parents/BP_Tank.Hull` (`self.Tank`)) (`self.Socket`) "SnapToTarget" "SnapToTarget" "SnapToTarget"))

(fn `Add HUD`
  (params (Owner :type "PlayerController Object Reference"))
  (returns (Widget :type "Widget Object Reference"))
  (bind _widget (`/Game/Magnus/Tank/Components/Actor_Components/AC_Weapon.Add HUD` (`self.Weapon`) Owner))
  (return _widget))

(fn `Clamp Elevation`
  (params (`Axis Input` :type "Float (double-precision)"))
  (returns (Elevation :type "Float (double-precision)"))
  (bind _output_get (set `self.Elevation` (`KismetMathLibrary.FClamp` `Axis Input` (`self.Min Elevation`) (`self.Max Elevation`))))
  (return _output_get))

(fn `Muzzle Hitscan`
  (returns (Hit :type Boolean) (`Impact Point` :type "Vector Structure"))
  (bind (_returnvalue_location _returnvalue_rotation) (`KismetMathLibrary.BreakTransform` (`SceneComponent.GetSocketTransform` (`self.Cannon`) "Muzzle" "RTS_World")))
  (bind (_outhit _returnvalue) (`KismetSystemLibrary.LineTraceSingle` _returnvalue_location (+ _returnvalue_location (* (`KismetMathLibrary.GetForwardVector` _returnvalue_rotation) (`self.Ray Length`))) "TraceTypeQuery2"))
  (return _returnvalue (`.ImpactPoint` (`GameplayStatics.BreakHitResult` _outhit))))

(fn `Scope Elevate`
  (params (`Axis Input` :type "Float (double-precision)"))
  (returns (Angle :type "Float (double-precision)"))
  (bind _angle (`self.Set Elevate` (+ (* `Axis Input` (`self.Movement Speed`)) (`self.Elevation`))))
  (return _angle))

(fn `Scope Rotate`
  (params (`Axis Input` :type "Float (double-precision)"))
  (returns (Angle :type "Float (double-precision)"))
  (if (`self.Artillery`)
    (`/Game/Parents/BP_Tank.Turn Right` (`self.Tank`) `Axis Input`)
    (else
      (bind _angle (`self.Set Rotate` (+ (* `Axis Input` (`self.Movement Speed`)) (`self.Rotation`))))
      (return _angle))))

(fn `Set Elevate`
  (params (`Axis Input` :type "Float (double-precision)"))
  (returns (Angle :type "Float (double-precision)"))
  (bind _elevation (`self.Clamp Elevation` `Axis Input`))
  (`SceneComponent.K2_SetRelativeRotation` (`self.Elevator`) (`KismetMathLibrary.MakeRotator` 0.0 _elevation) false false)
  (return _elevation))

(fn `Set Orientation`
  (params (Elevation :type "Float (double-precision)") (Rotation :type "Float (double-precision)"))
  (if (not (`self.Artillery`))
    (`self.Set Elevate` Elevation)
    (`self.Set Rotate` Rotation)))

(fn `Set Rotate`
  (params (`Axis Input` :type "Float (double-precision)"))
  (returns (Angle :type "Float (double-precision)"))
  (bind _output_get (set `self.Rotation` (select `bool` (> (`self.Max Rotation`) 0.0) :`false` `Axis Input` :`true` (`KismetMathLibrary.FClamp` `Axis Input` (`self.Min Rotation`) (`self.Max Rotation`)))))
  (`SceneComponent.K2_SetRelativeRotation` (`self.Rotator`) (`KismetMathLibrary.MakeRotator` 0.0 0.0 _output_get) false false)
  (return _output_get))

(fn `UserConstructionScript`
  (set `self.Rotator` (`self.Base`))
  (set `self.Elevator` (`self.Pivot 2`)))