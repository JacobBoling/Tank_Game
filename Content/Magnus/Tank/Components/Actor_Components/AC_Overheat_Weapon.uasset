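; Weapon component for tank turrets that builds heat with each shot and locks out firing when it overheats.
; Successful parent fire calls add heat and spin the optional Spinner mesh, while Release starts delayed cooling on Tick.
; Reaching max heat forces the turret to release and starts a timer that clears the lockout.
; It creates an overheat HUD widget and updates reticle progress and color from the heat state.
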(event `self.Release`
  (`parent.Release`)
  (`KismetSystemLibrary.Delay` (`self.Cooldown Delay`))
  (set `self.Cooling` true))

(event `Begin Overheat`
  (set `self.Overheated` true)
  (`/Game/Parents/BP_Turret.Release` (`self.Turret`))
  (bind _returnvalue (`KismetSystemLibrary.K2_SetTimerDelegate` (delegate `End Overheat`) (`self.Overheat Delay`)))
  (set `self.Overheat Timer` _returnvalue))

(event `End Overheat`
  (set `self.Overheated` false))

(event `self.ReceiveTick`
  (params (DeltaSeconds :type "Float (single-precision)"))
  (set `self.Reticle Progress` (`self.Heat Percentage`))
  (set `self.Reticle Color` (select `bool` (`self.Overheated`) :`false` (struct :`R` 1.0 :`G` 1.0 :`B` 1.0 :`A` 1.0) :`true` (struct :`R` 1.0 :`A` 1.0) :!type "LinearColor Structure"))
  (if (`self.Cooling`)
    (set `self.Heat` (`KismetMathLibrary.FClamp` (- (`self.Heat`) (`self.Cooldown Increment`)) 0.0 (`self.Max Heat`)))))

(event `Spin Up`
  (params (Spin :type "Float (double-precision)"))
  (bind _output_get (set `self.Spin` Spin))
  (`SceneComponent.K2_AddRelativeRotation` (`self.Spinner`) (`KismetMathLibrary.MakeRotator` _output_get) false false))

(fn `Add HUD`
  (params (Controller :type "PlayerController Object Reference"))
  (returns (Widget :type "Widget Object Reference"))
  (`parent.Add HUD` Controller)
  (bind _returnvalue (`|CreateWidget` "/Game/Magnus/Tank/Components/Widgets/WBP_HUD_Overheat.WBP_HUD_Overheat_C" Controller))
  (bind _output_get (set `self.HUD Overheat Ref` _returnvalue))
  (`UserWidget.AddToViewport` _output_get 0)
  (set `/Game/Magnus/Tank/Components/Widgets/WBP_HUD_Overheat.Weapon` self _output_get)
  (return _output_get))

(fn `Fire`
  (returns (Return :type Boolean))
  (bind _spinner (`self.Spinner`))
  (if (not (`self.Overheated`))
    (`/Engine/EditorBlueprintResources/StandardMacros.IsValid` _spinner
      (:`Is Valid`
        (`SceneComponent.K2_AddRelativeRotation` _spinner (`KismetMathLibrary.MakeRotator` (`self.Spin`)) false false))
      (:`Is Not Valid`
        _))
    (bind _return (`parent.Fire`))
    (if _return
      (bind _output_get (set `self.Heat` (+ (`self.Heat`) (`self.Heat Increment`))))
      (set `self.Cooling` false))
    (if (>= _output_get (`self.Max Heat`))
      (`self.Begin Overheat`)
      (return false)
      (else
        (return true)))))