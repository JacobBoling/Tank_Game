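; Parent tank pawn with movement, health and a swappable child-actor turret that number keys switch between five weapon types.
; Enhanced Input drives frame-scaled movement, scrolling tread material UVs, firing and scoped view.
; Outside scope and artillery modes, a player's camera trace steers the turret at constant speed.
; Zero health triggers death, which for players reports the kill, applies a destroyed overlay and enters a timed respawn overview.
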(event `self.ReceiveBeginPlay`
  (set `self.Health` (`self.Max Health`)))

(event `self.ReceivePossessed`
  (params (NewController :type "Controller Object Reference"))
  (bind _player_controller (`self.Player Controller`))
  (bind _asbp_tank_controller (cast `/Game/Magnus/BP_Tank_Controller` NewController))
  (bind _output_get (set `self.Player Controller` _asbp_tank_controller))
  (set `self.Is Player` true)
  (bind _asbp_tank_hud (cast `/Game/Magnus/BP_Tank_HUD` (`PlayerController.GetHUD` _output_get)))
  (bind _output_get_2 (set `self.HUD` _asbp_tank_hud))
  (`/Game/Magnus/BP_Tank_HUD.Set Tank` _output_get_2 self)
  (bind _asbp_tank_player_state (cast `/Game/Menus/BP_Tank_Player_State` (`Controller.PlayerState` (`self.Player Controller`))))
  (set `self.Player Team` (`/Game/Menus/BP_Tank_Player_State.Team` _asbp_tank_player_state))
  (set `self.Player Name` (`/Game/Menus/BP_Tank_Player_State.Name` _asbp_tank_player_state))
  (`WidgetBlueprintLibrary.SetInputMode_GameOnly` _player_controller)
  (message `EnhancedInputSubsystemInterface.AddMappingContext` (pcsubsystem `EnhancedInputLocalPlayerSubsystem` _player_controller) "/Game/Inputs/IMC_Tank.IMC_Tank" 0 (struct)))

(event `Is Target`
  (if (not (`self.Is Player`))
    (bind _returnvalue (`|CreateWidget` "/Game/Magnus/Tank/Components/Widgets/WBP_Health_Bar.WBP_Health_Bar_C" null self "Target"))
    (`WidgetComponent.SetWidget` (`self.Health Bar Container`) _returnvalue)))

(event `self.Modify Health`
  (params (Instigator :type "Pawn Object Reference") (Damage :type "Float (double-precision)") (Type :type "/Game/Magnus/Tank/Components/E_Damage_Type Enum" :default "NewEnumerator5"))
  (if (`self.Alive`)
    (bind _output_get (set `self.Health` (`KismetMathLibrary.FClamp` (- (`self.Health`) Damage) 0.0 (`self.Max Health`))))
    (if (== _output_get 0.0)
      (bind _asbp_tank (cast `/Game/Parents/BP_Tank` Instigator))
      (`self.Die` _asbp_tank Type))))

(event `self.Die`
  (params (KIller :type "/Game/Parents/BP_Tank Object Reference") (`Damage Type` :type "/Game/Magnus/Tank/Components/E_Damage_Type Enum" :default "NewEnumerator5"))
  (set `self.Alive` false)
  (if (`self.Is Player`)
    (`/Game/Magnus/BP_Tank_HUD.Remove HUD` (`self.HUD`))
    (`self.DisableInput` (`self.Player Controller`))
    (message `/Game/Magnus/BI_Game_Functions.Record Kill` (`GameplayStatics.GetGameMode`) (make `/Game/Magnus/Tank/Components/F_Kill_Event` KIller self `Damage Type`))
    (`self.SetLifeSpan` 5.0)
    (for _array_element (`self.Meshes`)
      (`MeshComponent.SetOverlayMaterial` _array_element "/Game/Magnus/Materials/M_Destroyed.M_Destroyed")
      (`KismetSystemLibrary.Delay` 1.0)
      (`/Game/Magnus/BP_Tank_Controller.Enter Overview` (`self.Player Controller`) "Spawn" 5.0))))

(event `Key|One`
  (params (Key :type "Key Structure"))
  (:`Pressed`
    (`self.Change Turret` "/Game/Magnus/Tank/Turrets/BP_Standard.BP_Standard_C")))

(event `Move Camera`
  (params (Location :type "Vector Structure"))
  (`SceneComponent.K2_SetRelativeLocation` (`self.Camera Holder`) Location false false))

(event `Change Turret`
  (params (Turret :type "/Game/Parents/BP_Turret Class Reference"))
  (bind _turret_container (`self.Turret Container`))
  (`ChildActorComponent.SetChildActorClass` _turret_container Turret)
  (bind _asbp_turret (cast `/Game/Parents/BP_Turret` (`ChildActorComponent.ChildActor` _turret_container)))
  (bind _output_get (set `self.Turret` _asbp_turret))
  (set `/Game/Parents/BP_Turret.Tank` self _output_get))

(event `Key|Two`
  (params (Key :type "Key Structure"))
  (:`Pressed`
    (`self.Change Turret` "/Game/Magnus/Tank/Turrets/BP_Minigun.BP_Minigun_C")))

(event `EnhancedInput|/Game/Inputs/IA_Forward`
  (params (ActionValue :type "Float (double-precision)") (ElapsedSeconds :type "Float (double-precision)") (TriggeredSeconds :type "Float (double-precision)") (InputAction :type "InputAction Object Reference" :default "/Game/Inputs/IA_Forward.IA_Forward"))
  (:`Triggered`
    (`self.Move Forward` ActionValue)))

(event `EnhancedInput|/Game/Inputs/IA_Turn_Right`
  (params (ActionValue :type "Float (double-precision)") (ElapsedSeconds :type "Float (double-precision)") (TriggeredSeconds :type "Float (double-precision)") (InputAction :type "InputAction Object Reference" :default "/Game/Inputs/IA_Turn_Right.IA_Turn_Right"))
  (:`Triggered`
    (`self.Turn Right` ActionValue)))

(event `Key|Three`
  (params (Key :type "Key Structure"))
  (:`Pressed`
    (`self.Change Turret` "/Game/Magnus/Tank/Turrets/BP_Tank_Destroyer.BP_Tank_Destroyer_C")))

(event `Key|Four`
  (params (Key :type "Key Structure"))
  (:`Pressed`
    (`self.Change Turret` "/Game/Magnus/Tank/Turrets/BP_Artillery.BP_Artillery_C")))

(event `EnhancedInput|/Game/Inputs/IA_Look_Up`
  (params (ActionValue :type "Float (double-precision)") (ElapsedSeconds :type "Float (double-precision)") (TriggeredSeconds :type "Float (double-precision)") (InputAction :type "InputAction Object Reference" :default "/Game/Inputs/IA_Look_Up.IA_Look_Up"))
  (:`Triggered`
    (if (`self.Scoped`)
      (bind _angle (`/Game/Parents/BP_Turret.Scope Elevate` (`self.Turret`) ActionValue))
      (`SceneComponent.K2_SetRelativeRotation` (`self.Camera Holder`) (`KismetMathLibrary.MakeRotator` 0.0 _angle (stale `EnhancedInput|/Game/Inputs/IA_Look_Right` _angle)) false false :!label _label)
      (else
        (`SceneComponent.K2_AddRelativeRotation` (`self.Camera Holder`) (`KismetMathLibrary.MakeRotator` 0.0 ActionValue (stale `EnhancedInput|/Game/Inputs/IA_Look_Right` ActionValue)) false false :!label _label_2)))))

(event `EnhancedInput|/Game/Inputs/IA_Zoom`
  (params (ActionValue :type Boolean) (ElapsedSeconds :type "Float (double-precision)") (TriggeredSeconds :type "Float (double-precision)") (InputAction :type "InputAction Object Reference" :default "/Game/Inputs/IA_Zoom.IA_Zoom"))
  (:`Triggered`
    (`PlayerController.SetViewTargetWithBlend` (`self.Player Controller`) (`self.Turret`) 0.01 "VTBlend_Linear" 0.0 false)
    (set `self.Scoped` ActionValue :!label _label_3))
  (:`Completed`
    (`PlayerController.SetViewTargetWithBlend` (`self.Player Controller`) self 0.01 "VTBlend_Linear" 0.0 false)
    (goto _label_3)))

(event `Key|Five`
  (params (Key :type "Key Structure"))
  (:`Pressed`
    (`self.Change Turret` "/Game/Magnus/Tank/Turrets/BP_Flamethrower.BP_Flamethrower_C")))

(event `EnhancedInput|/Game/Inputs/IA_Look_Right`
  (params (ActionValue :type "Float (double-precision)") (ElapsedSeconds :type "Float (double-precision)") (TriggeredSeconds :type "Float (double-precision)") (InputAction :type "InputAction Object Reference" :default "/Game/Inputs/IA_Look_Right.IA_Look_Right"))
  (:`Triggered`
    (if (`self.Scoped`)
      (bind _angle (`/Game/Parents/BP_Turret.Scope Rotate` (`self.Turret`) ActionValue))
      (goto _label)
      (else
        (goto _label_2)))))

(event `EnhancedInput|/Game/Inputs/IA_Scroll`
  (params (ActionValue :type "Float (double-precision)") (ElapsedSeconds :type "Float (double-precision)") (TriggeredSeconds :type "Float (double-precision)") (InputAction :type "InputAction Object Reference" :default "/Game/Inputs/IA_Scroll.IA_Scroll"))
  (:`Triggered`
    (if (`/Game/Parents/BP_Turret.Artillery` (`self.Turret`))
      (`/Game/Parents/BP_Turret.Scope Elevate` (`self.Turret`) (* ActionValue -1.0)))))

(event `self.ReceiveTick`
  (params (DeltaSeconds :type "Float (single-precision)"))
  (if (and (not (`/Game/Parents/BP_Turret.Artillery` (`self.Turret`))) (not (`self.Scoped`)) (`self.Is Player`))
    (bind (_hit_found _impact_point) (`self.Camera Trace`))
    (`self.Aim` _hit_found _impact_point DeltaSeconds)))

(event `EnhancedInput|/Game/Inputs/IA_Fire`
  (params (ActionValue :type Boolean) (ElapsedSeconds :type "Float (double-precision)") (TriggeredSeconds :type "Float (double-precision)") (InputAction :type "InputAction Object Reference" :default "/Game/Inputs/IA_Fire.IA_Fire"))
  (:`Triggered`
    (`/Game/Parents/BP_Turret.Fire` (`self.Turret`)))
  (:`Completed`
    (`/Game/Parents/BP_Turret.Release` (`self.Turret`))))

(fn `Aim`
  (params (Condition :type Boolean) (Position :type "Vector Structure (by ref)") (`Delta Time` :type "Float (single-precision)"))
  (locals (`Aiming Socket` :type Name :default "Cannon"))
  (bind (_returnvalue_roll _returnvalue_pitch _returnvalue_yaw) (`KismetMathLibrary.BreakRotator` (`KismetMathLibrary.InverseTransformRotation` (`self.GetTransform`) (`KismetMathLibrary.RInterpTo_Constant` (`SceneComponent.GetSocketRotation` (`/Game/Parents/BP_Turret.Pivot 2` (`self.Turret`)) (`local.Aiming Socket`)) (`self.Target Rotation`) `Delta Time` (* (`/Game/Parents/BP_Turret.Movement Speed` (`self.Turret`)) 50.0)))))
  (if Condition
    (set `self.Target Rotation` (`KismetMathLibrary.FindLookAtRotation` (`SceneComponent.GetSocketLocation` (`/Game/Parents/BP_Turret.Pivot 2` (`self.Turret`)) (`local.Aiming Socket`)) Position))
    (else
      (set `self.Target Rotation` (`.Rotation` (`Controller.GetPlayerViewPoint` (`self.GetController`))))))
  (`/Game/Parents/BP_Turret.Set Orientation` (`self.Turret`) _returnvalue_pitch _returnvalue_yaw))

(fn `Camera Trace`
  (returns (`Hit Found` :type Boolean) (`Impact Point` :type "Vector Structure"))
  (bind (_returnvalue_location _returnvalue_rotation) (`KismetMathLibrary.BreakTransform` (`SceneComponent.K2_GetComponentToWorld` (`self.Camera`))))
  (bind (_outhit _returnvalue) (`KismetSystemLibrary.LineTraceSingle` _returnvalue_location (+ _returnvalue_location (* (`KismetMathLibrary.GetForwardVector` _returnvalue_rotation) 2000000.0)) "TraceTypeQuery1" false (`|MakeArray` (`self.Turret`) :!type "Actor Object Reference")))
  (return _returnvalue (`.ImpactPoint` (`GameplayStatics.BreakHitResult` _outhit))))

(fn `Move Forward`
  (params (Input :type "Float (double-precision)"))
  (bind _movement (`self.Input to Movement` Input (`self.Forward Speed`)))
  (`self.K2_AddActorLocalOffset` (`KismetMathLibrary.MakeVector` _movement))
  (set `self.Position Offset` (* (`self.Forward Fudge Factor`) _movement))
  (`self.UpdateTreadUVs`))

(fn `Turn Right`
  (params (Input :type "Float (double-precision)"))
  (bind _movement (`self.Input to Movement` Input (`self.Turn Speed`)))
  (`self.K2_AddActorLocalRotation` (`KismetMathLibrary.MakeRotator` 0.0 0.0 _movement))
  (set `self.Turn Offset` (* (`self.Turn Fudge Factor`) _movement))
  (`self.UpdateTreadUVs`)
  (`SceneComponent.K2_AddRelativeRotation` (`self.Camera Holder`) (`KismetMathLibrary.MakeRotator` 0.0 0.0 (* _movement -1.0)) false false))

(fn `UpdateTreadUVs`
  (bind _returnvalue (* (`self.Tread Width`) -1.0))
  (bind _output_get (set `self.Offset L` (+ (`self.Offset L`) (`self.Position Offset`) (`self.Turn Offset`))))
  (set `self.UV Offset L` (/ _output_get _returnvalue))
  (bind _output_get_2 (set `self.Offset R` (+ (`self.Offset R`) (`self.Position Offset`) (* (`self.Turn Offset`) -1.0))))
  (set `self.UV Offset R` (/ _output_get_2 _returnvalue))
  (`MeshComponent.SetScalarParameterValueOnMaterials` (`self.Tread L`) "TreadUVOffset" (`self.UV Offset L`))
  (`MeshComponent.SetScalarParameterValueOnMaterials` (`self.Tread R`) "TreadUVOffset" (`self.UV Offset R`)))

(fn `UserConstructionScript`
  (`self.Change Turret` (`self.Turret Class`))
  (bind _output_get (set `self.Meshes` (`self.K2_GetComponentsByClass` "/Script/Engine.StaticMeshComponent")))
  (`KismetArrayLibrary.Array_Append` _output_get (`self.K2_GetComponentsByClass` (`self.Turret`) "/Script/Engine.StaticMeshComponent"))
  (for _array_element (`self.Meshes`)
    (`PrimitiveComponent.CreateDynamicMaterialInstance` _array_element 0 (`PrimitiveComponent.GetMaterial` _array_element 0) "None"))
  (if (!= (`self.Tread L`) null)
    (bind _returnvalue (`PrimitiveComponent.CreateDynamicMaterialInstance` (`self.Tread L`) 0 "/Game/Magnus/Tank/Material_Instances/MI_Tread.MI_Tread" "None"))
    (set `self.Tread Material L` _returnvalue)
    (bind _returnvalue_2 (`PrimitiveComponent.CreateDynamicMaterialInstance` (`self.Tread R`) 0 "/Game/Magnus/Tank/Material_Instances/MI_Tread.MI_Tread" "None"))
    (set `self.Tread Material R` _returnvalue_2)))