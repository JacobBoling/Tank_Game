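; Lobby game mode that marks the host, greets joining players and launches the match.
; On BeginPlay it flags the first player's BP_Tank_Player_State as host.
; New players' BP_Lobby_Controller gets its OnPlayerJoin dispatcher called, then bound.
; StartMatch issues a ServerTravel console command using the map stored in BP_Lobby_State; logout is empty and the host-based session teardown is unconnected.
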(event `self.ReceiveBeginPlay`
  (bind _asbp_tank_player_state (cast `/Game/Menus/BP_Tank_Player_State` (`GameplayStatics.GetPlayerState` 0)))
  (bind _output_get (set `self.Host Player` _asbp_tank_player_state))
  (set `/Game/Menus/BP_Tank_Player_State.Host` true _output_get))

(event `self.HandleStartingNewPlayer`
  (params (NewPlayer :type "PlayerController Object Reference"))
  (bind _asbp_lobby_controller (cast `/Game/Menus/BP_Lobby_Controller` NewPlayer))
  (`self.On Player Join` _asbp_lobby_controller)
  (add `self.On Player Join` self (`|CreateDelegate` _asbp_lobby_controller :!event `Auto Receive Login`)))

(event `Start Match`
  (bind _asbp_lobby_state (cast `/Game/Menus/BP_Lobby_State` (`GameplayStatics.GetGameState`)))
  (`KismetSystemLibrary.ExecuteConsoleCommand` (`KismetStringLibrary.BuildString_Name` "" "ServerTravel " (`/Game/Menus/BP_Lobby_State.Map` _asbp_lobby_state)) null))

(event `self.K2_OnSwapPlayerControllers`
  (params (OldPC :type "PlayerController Object Reference") (NewPC :type "PlayerController Object Reference")))

(event `self.K2_OnLogout`
  (params (ExitingController :type "Controller Object Reference")))

(fn `UserConstructionScript`)