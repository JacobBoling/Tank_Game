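; Flame projectile that sticks to what it hits and deals damage over time.
; On first hit, it snaps to the impact point, attaches to the hit component and switches its hitbox to overlap.
; Overlapping a BI_Damageable actor stores it as the single target and starts a looping damage timer, cleared when that target leaves.
; After its contact lifetime, the fire deactivates, the hitbox ignores collisions and a short lifespan is set.
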(event `self.Hitbox Sphere.OnComponentHit`
  (params (HitComponent :type "PrimitiveComponent Object Reference") (OtherActor :type "Actor Object Reference") (OtherComp :type "PrimitiveComponent Object Reference") (NormalImpulse :type "Vector Structure") (Hit :type "HitResult Structure (by ref)"))
  (`/Engine/EditorBlueprintResources/StandardMacros.DoOnce` false
    (:`Completed`
      (`self.K2_AddActorLocalOffset` (- (`.ImpactPoint` (`GameplayStatics.BreakHitResult` Hit)) (`self.K2_GetActorLocation`)))
      (`self.K2_AttachToComponent` OtherComp "None" "KeepWorld" "KeepWorld" "KeepWorld")
      (`PrimitiveComponent.SetCollisionResponseToAllChannels` (`self.Hitbox Sphere`) "ECR_Overlap")
      (`KismetSystemLibrary.K2_SetTimerDelegate` (delegate `Extinguish`) (`self.Contact Lifetime`) true))))

(event `Extinguish`
  (`ActorComponent.Deactivate` (`self.Fire`))
  (`PrimitiveComponent.SetCollisionResponseToAllChannels` (`self.Hitbox Sphere`) "ECR_Ignore")
  (`self.SetLifeSpan` 2.0))

(event `self.ReceiveActorBeginOverlap`
  (params (OtherActor :type "Actor Object Reference"))
  (if (`KismetSystemLibrary.DoesImplementInterface` OtherActor "/Game/Magnus/Tank/Components/BI_Damageable.BI_Damageable_C")
    (set `self.Target` OtherActor)
    (bind _returnvalue (`KismetSystemLibrary.K2_SetTimerDelegate` (delegate `Damage Over Time`) 1.0 true))
    (set `self.Damage Timer` _returnvalue)))

(event `Damage Over Time`
  (message `/Game/Magnus/Tank/Components/BI_Damageable.Modify Health` (`self.Target`) (`self.Instigator`) 0.5 "NewEnumerator5"))

(event `self.ReceiveActorEndOverlap`
  (params (OtherActor :type "Actor Object Reference"))
  (if (== OtherActor (`self.Target`))
    (`KismetSystemLibrary.K2_ClearAndInvalidateTimerHandle` (`self.Damage Timer`))))

(fn `UserConstructionScript`
  (`parent.UserConstructionScript`))