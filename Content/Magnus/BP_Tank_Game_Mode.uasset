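; Game mode for a tank game that runs match flow and relays kill and spawn events.
; Chained timers move from preround through a timed round, scheduled only when RoundLength is positive, to postround and a ServerTravel back to Lobby.
; Round end fires the EndGame dispatcher, while RecordKill and TankSpawn pass their data on through killfeed and tank-spawn notifications.
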(event `Initialize Game`
  (`KismetSystemLibrary.K2_SetTimerDelegate` (delegate `Start Game`) (`self.Preround Length`)))

(event `Start Game`
  (if (> (`self.Round Length`) 0.0)
    (bind _returnvalue (`KismetSystemLibrary.K2_SetTimerDelegate` (delegate `End Game`) (`self.Round Length`)))
    (set `self.Round Timer` _returnvalue)))

(event `End Game`
  (`self.Dispatch End Game`)
  (`KismetSystemLibrary.K2_SetTimerDelegate` (delegate `Return to Lobby`) (`self.Postround Length`)))

(event `Return to Lobby`
  (`KismetSystemLibrary.ExecuteConsoleCommand` (`KismetStringLibrary.BuildString_Name` "" "ServerTravel " "Lobby") null))

(event `/Game/Magnus/BI_Game_Functions.Record Kill`
  (params (`Kill Event` :type "/Game/Magnus/Tank/Components/F_Kill_Event Structure"))
  (`self.Notify Killfeeds` `Kill Event`))

(event `/Game/Magnus/BI_Game_Functions.Tank Spawn`
  (params (`New Tank` :type "/Game/Parents/BP_Tank Object Reference"))
  (`self.Notify Tank Spawn` `New Tank`))

(fn `UserConstructionScript`)