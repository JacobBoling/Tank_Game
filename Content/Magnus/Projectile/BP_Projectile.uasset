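; BP_Projectile is a projectile actor that applies impact damage to what it hits.
; The construction script calls SetValues, which sets the movement component's initial speed from MuzzleVelocity and scales the actor from Radius.
; When HitboxSphere registers a hit, it sends ModifyHealthMessage to the other actor with the damage and instigator, then destroys itself.
; A debug hit print and a hit-indicator spawn are present but disconnected.
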(event `Set Values`
  (set `ProjectileMovementComponent.InitialSpeed` (`self.Muzzle Velocity`) (`self.ProjectileMovement`))
  (`self.SetActorRelativeScale3D` (`KismetMathLibrary.Conv_DoubleToVector` (/ (`self.Radius`) 50.0))))

(event `self.Hitbox Sphere.OnComponentHit`
  (params (HitComponent :type "PrimitiveComponent Object Reference") (OtherActor :type "Actor Object Reference") (OtherComp :type "PrimitiveComponent Object Reference") (NormalImpulse :type "Vector Structure") (Hit :type "HitResult Structure (by ref)"))
  (message `/Game/Magnus/Tank/Components/BI_Damageable.Modify Health` OtherActor (`self.Impact Damage`) (`self.Instigator`))
  (`self.K2_DestroyActor`))

(fn `UserConstructionScript`
  (`self.Set Values`))