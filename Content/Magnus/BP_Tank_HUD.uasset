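; Tank HUD that draws a white screen-space polyline through an array of world-space Points, which is not filled within this Blueprint.
; Each DrawHUD, if Points differs from the Empty array, it removes the first point.
; It then projects each remaining consecutive pair through PlayerOwner to screen coordinates and connects them with DrawLine.
; The removal mutates the stored array, so the line loses a point per draw unless Points is refreshed.
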(event `self.ReceiveDrawHUD`
  (params (SizeX :type Integer) (SizeY :type Integer))
  (bind _points (`self.Points`))
  (bind _playerowner (`self.PlayerOwner`))
  (if (not (`KismetArrayLibrary.Array_Identical` (`self.Points`) (`self.Empty`)))
    (`KismetArrayLibrary.Array_Remove` _points)
    (for (_array_element _array_index) _points
      (if (< _array_index (- (`KismetArrayLibrary.Array_Length` _points) 1))
        (bind _screenposition (`GameplayStatics.ProjectWorldToScreen` _playerowner _array_element))
        (bind _screenposition_2 (`GameplayStatics.ProjectWorldToScreen` _playerowner (`|GetArrayItem` (`self.Points`) (+ _array_index 1))))
        (`self.DrawLine` (`KismetMathLibrary.BreakVector2D` _screenposition) (`.Y` (`KismetMathLibrary.BreakVector2D` _screenposition)) (`KismetMathLibrary.BreakVector2D` _screenposition_2) (`.Y` (`KismetMathLibrary.BreakVector2D` _screenposition_2)) (struct :`R` 1.0 :`G` 1.0 :`B` 1.0 :`A` 1.0) 5.0)))))

(fn `UserConstructionScript`)