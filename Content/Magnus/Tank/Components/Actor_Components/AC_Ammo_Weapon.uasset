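; AC_Ammo_Weapon is a tank weapon actor component that adds limited ammunition to the firing behavior of its parent weapon component.
; On BeginPlay it runs the parent logic, then fills Ammo from MaxAmmo.
; Its Fire override calls the parent Fire only while ammo remains, spends one round when that succeeds, and returns whether a shot was fired.
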(event `self.ReceiveBeginPlay`
  (`parent.ReceiveBeginPlay`)
  (set `self.Ammo` (`self.Max Ammo`)))

(fn `Fire`
  (returns (Return :type Boolean))
  (if (> (`self.Ammo`) 0)
    (bind _return (`parent.Fire`))
    (if _return
      (set `self.Ammo` (- (`self.Ammo`) 1))
      (return true)
      (else
        _)))
  (return false))