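; BP_Rocket_Projectile is a rocket projectile that runs a thruster for a limited time after it spawns.
; While the thruster is on, Tick calls the parent tick and then adds Thrust to HitboxSphere as a force on the X axis only.
; A one-shot timer set on BeginPlay switches the thruster off after ThrusterDuration, ending the push.
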(event `self.ReceiveBeginPlay`
  (`KismetSystemLibrary.K2_SetTimerDelegate` (delegate `End Thrust`) (`self.Thruster Duration`)))

(event `End Thrust`
  (set `self.Thruster On` false))

(event `self.ReceiveTick`
  (params (DeltaSeconds :type "Float (single-precision)"))
  (`parent.ReceiveTick` DeltaSeconds)
  (if (`self.Thruster On`)
    (`PrimitiveComponent.AddForce` (`self.Hitbox Sphere`) (`KismetMathLibrary.MakeVector` (`self.Thrust`)) "None" false)))

(fn `UserConstructionScript`
  (`parent.UserConstructionScript`))