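; BP_Drivetrain is a parent tank drivetrain that mounts six wheel or tread assemblies to the hull and animates tread movement.
; Construction fills SocketMountMap by pairing its socket keys, in order, with front, mid and rear mount components on each side.
; SetTank snaps each mount to its hull socket.
; UpdateUVs accumulates per-side offsets from position and opposing turn input, scaled by tread size, to scroll the tread materials.
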(event `self.Set Tank`
  (params (Tank :type "/Game/Parents/BP_Tank Object Reference"))
  (`parent.Set Tank` Tank)
  (bind _keys (`BlueprintMapLibrary.Map_Keys` (`self.Socket-Mount Map`)))
  (for _array_element _keys
    (`SceneComponent.K2_AttachToComponent` (`BlueprintMapLibrary.Map_Find` (`self.Socket-Mount Map`) _array_element) (`/Game/Parents/BP_Tank.Hull` (`self.Tank`)) _array_element "SnapToTarget" "SnapToTarget" "SnapToTarget" true)))

(event `Update UVs`
  (params (Position :type "Float (single-precision)") (Turn :type "Float (single-precision)"))
  (bind _returnvalue (* (`self.Tread Width + Thickness`) -1.0))
  (bind _output_get (set `self.Offset L` (+ Position Turn (`self.Offset L`))))
  (bind _returnvalue_2 (/ _output_get _returnvalue))
  (`MeshComponent.SetScalarParameterValueOnMaterials` (`self.Left Front Tread`) "TreadUVOffset" _returnvalue_2)
  (`MeshComponent.SetScalarParameterValueOnMaterials` (`self.Left Mid Tread`) "TreadUVOffset" _returnvalue_2)
  (`MeshComponent.SetScalarParameterValueOnMaterials` (`self.Left Rear Tread`) "TreadUVOffset" _returnvalue_2)
  (bind _output_get_2 (set `self.Offset R` (+ (`self.Offset R`) Position (* Turn -1.0))))
  (bind _returnvalue_3 (/ _output_get_2 _returnvalue))
  (`MeshComponent.SetScalarParameterValueOnMaterials` (`self.Right Front Tread`) "TreadUVOffset" _returnvalue_3)
  (`MeshComponent.SetScalarParameterValueOnMaterials` (`self.Right Mid Tread`) "TreadUVOffset" _returnvalue_3)
  (`MeshComponent.SetScalarParameterValueOnMaterials` (`self.Right Rear Tread`) "TreadUVOffset" _returnvalue_3))

(fn `UserConstructionScript`
  (`parent.UserConstructionScript`)
  (bind _keys (`BlueprintMapLibrary.Map_Keys` (`self.Socket-Mount Map`)))
  (for (_array_element _array_index) _keys
    (`BlueprintMapLibrary.Map_Add` (`self.Socket-Mount Map`) _array_element (`|GetArrayItem` (`|MakeArray` (`self.Left Front Mount`) (`self.Right Front Mount`) (`self.Left Mid Mount`) (`self.Right Mid Mount`) (`self.Left Rear Mount`) (`self.Right Rear Mount`) :!type "SceneComponent Object Reference") _array_index))))