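; Lobby player controller that shows the mouse cursor and drives the lobby menu's player list and map display.
; InitializePlayerList stores the local player state, creates the menu through BP_Lobby_HUD, adds existing players from the GameState, then initializes the menu.
; AutoReceiveLogin adds newly joined players through the same AddOtherPlayer filter, which skips the local player.
; SetMap forwards the map image and name to the menu.
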(event Custom|Auto%20Receive%20Login
  (params (New%20Player :type BP%20Lobby%20Controller%20Object%20Reference))
  (CallFunction|AddOtherPlayer (Variables|/Script/Engine.Controller|GetPlayerState New%20Player)))

(event Custom|Initialize%20Player%20List
  (params (State :type BP%20Tank%20Player%20State%20Object%20Reference))
  (Variables|Default|SetState State)
  (bind _asbp_lobby_hud (Utilities|Casting|CastToBP_Lobby_HUD (HUD|GetHUD)))
  (bind _lobby_menu (Default|InitializeHUDMenu _asbp_lobby_hud))
  (Variables|Default|SetLobby%20Menu _lobby_menu)
  (for _array_element (Variables|/Script/Engine.GameStateBase|GetPlayerArray (Game|GetGameState))
    (CallFunction|AddOtherPlayer _array_element))
  (Default|InitializeMenu (Variables|Default|GetLobby%20Menu) (Variables|Default|GetState) (Game|GetGameState)))

(event Custom|Add%20Other%20Player
  (params (Player%20State :type Player%20State%20Object%20Reference))
  (if (!= Player%20State (Variables|Default|GetState))
    (Default|AddPlayerItem (Variables|Default|GetLobby%20Menu) Player%20State)))

(event Custom|Set%20Map
  (params (Image :type Slate%20Brush%20Structure) (Name :type Name))
  (Default|SetMap (Variables|Default|GetLobby%20Menu) Image Name))

(event EventBeginPlay
  (Variables|Default|SetbShowMouseCursor true))

(event Input|KeyboardEvents|DebugKeyT
  (params (Key :type Key%20Structure :default "None") (ActionValue :type Input%20Action%20Value%20Structure)))

(fn ConstructionScript)