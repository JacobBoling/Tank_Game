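; Lobby game state for a tank game that holds the selected map and checks player names and readiness.
; The construction script defaults Map to the first key in MapImages, and its RepNotify passes the map's name and image to each player's lobby controller.
; CheckName rejects names already used by another player state in PlayerArray.
; CheckReady sets MasterReady true only when every player is ready.
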(event `self.ReceiveBeginPlay`)

(fn `Check Name`
  (params (Name :type Text) (`Player State` :type "/Game/Menus/BP_Tank_Player_State Object Reference"))
  (returns (`Valid Name` :type Boolean))
  (for _array_element (`self.PlayerArray`)
    (bind _asbp_tank_player_state (cast `/Game/Menus/BP_Tank_Player_State` _array_element))
    (if (and (== (`/Game/Menus/BP_Tank_Player_State.Name` _asbp_tank_player_state) Name) (!= _asbp_tank_player_state `Player State`))
      (return false)))
  (return true))

(fn `Check Ready`
  (returns (Ready :type Boolean))
  (for _array_element (`self.PlayerArray`)
    (bind _asbp_tank_player_state (cast `/Game/Menus/BP_Tank_Player_State` _array_element))
    (if (not (`/Game/Menus/BP_Tank_Player_State.Ready` _asbp_tank_player_state))
      (bind _output_get (set `self.Master Ready` false))
      (return _output_get)))
  (bind _output_get_2 (set `self.Master Ready` true))
  (return _output_get_2))

(fn `OnRep_Map`
  (bind _map (`self.Map`))
  (for _array_element (`self.PlayerArray`)
    (bind _asbp_lobby_controller (cast `/Game/Menus/BP_Lobby_Controller` (`PlayerState.GetPlayerController` _array_element)))
    (`/Game/Menus/BP_Lobby_Controller.Change Map` _asbp_lobby_controller (`BlueprintMapLibrary.Map_Find` (`self.Map Images`) _map) _map)))

(fn `UserConstructionScript`
  (bind _keys (`BlueprintMapLibrary.Map_Keys` (`self.Map Images`)))
  (set `self.Map` (`|GetArrayItem` _keys)))