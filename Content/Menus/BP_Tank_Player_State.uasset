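; Player state for the multiplayer tank game, holding name, ready status, team, loadout and host flag.
; Server BeginPlay assigns a numbered name and sets ServerNotify, whose RepNotify initializes the lobby player list or, with game mode access, sets the tank controller's round timer and binds game mode events.
; Name changes and ready updates are checked through the lobby game state.
; CopyProperties carries loadout, team, host and name to the new player state.
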(event `self.ReceiveBeginPlay`
  (if (`KismetSystemLibrary.IsServer`)
    (set `self.Server Notify` true)
    (set `self.Name` (`|FormatText` "Player {Number}" (`GameplayStatics.GetNumPlayerStates`)))))

(event `Set Ready`
  (params (Ready :type Boolean))
  (set `self.Ready` Ready))

(event `Set Name`
  (params (Name :type Text))
  (bind _asbp_lobby_state (cast `/Game/Menus/BP_Lobby_State` (`GameplayStatics.GetGameState`)))
  (bind _valid_name (`/Game/Menus/BP_Lobby_State.Check Name` _asbp_lobby_state Name self))
  (if _valid_name
    (set `self.Name` Name)))

(event `self.ReceiveCopyProperties`
  (params (NewPlayerState :type "PlayerState Object Reference"))
  (bind _asbp_tank_player_state (cast `/Game/Menus/BP_Tank_Player_State` NewPlayerState))
  (set `/Game/Menus/BP_Tank_Player_State.Loadout` (`self.Loadout`) _asbp_tank_player_state)
  (set `/Game/Menus/BP_Tank_Player_State.Team` (`self.Team`) _asbp_tank_player_state)
  (set `/Game/Menus/BP_Tank_Player_State.Host` (`self.Host`) _asbp_tank_player_state)
  (set `/Game/Menus/BP_Tank_Player_State.Name` (`self.Name`) _asbp_tank_player_state))

(fn `OnRep_Ready`
  (bind _asbp_lobby_state (cast `/Game/Menus/BP_Lobby_State` (`GameplayStatics.GetGameState`)))
  (`/Game/Menus/BP_Lobby_State.Check Ready` _asbp_lobby_state))

(fn `OnRep_Server Notify`
  (bind _returnvalue (`self.GetPlayerController`))
  (`/Engine/EditorBlueprintResources/ActorMacros.Switch Has Authority`
    (:`Authority`
      (if (`self.Host`)
        (bind _asbp_lobby_controller (cast `/Game/Menus/BP_Lobby_Controller` _returnvalue :!label _label)
          (:`then`
            (`/Game/Menus/BP_Lobby_Controller.Initialize Player List` _asbp_lobby_controller self))
          (:`CastFailed`
            (bind _asbp_tank_controller (cast `/Game/Magnus/BP_Tank_Controller` _returnvalue))
            (bind _asbp_tank_game_mode (cast `/Game/Magnus/BP_Tank_Game_Mode` (`GameplayStatics.GetGameMode`)))
            (set `/Game/Magnus/BP_Tank_Controller.Round Timer` (`/Game/Magnus/BP_Tank_Game_Mode.Round Timer` _asbp_tank_game_mode) _asbp_tank_controller)
            (add `/Game/Magnus/BP_Tank_Game_Mode.Notify Killfeeds` _asbp_tank_game_mode (`|CreateDelegate` _asbp_tank_controller :!event `Notify Killfeed`))
            (add `/Game/Magnus/BP_Tank_Game_Mode.Dispatch End Game` _asbp_tank_game_mode (`|CreateDelegate` _asbp_tank_controller :!event `End Game`))
            (add `/Game/Magnus/BP_Tank_Game_Mode.Notify Tank Spawn` _asbp_tank_game_mode (`|CreateDelegate` _asbp_tank_controller :!event `Tank Spawn`))))))
    (:`Remote`
      (goto _label))))

(fn `UserConstructionScript`)