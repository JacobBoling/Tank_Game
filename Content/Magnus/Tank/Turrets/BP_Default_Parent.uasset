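; Default parent Blueprint for tank turrets, handling elevation and zoom camera placement.
; The construction script runs the parent's script, then moves the zoom camera to a fixed relative offset.
; Set Elevate clamps the axis input, then pitches Pivot1 for negative angles or Pivot2 otherwise, zeroing the other pivot, so depression and elevation rotate about separate points.
; It returns the clamped elevation.
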(fn `Set Elevate`
  (params (`Axis Input` :type "Float (double-precision)"))
  (returns (Angle :type "Float (double-precision)"))
  (locals (`Local Elevation` :type "Float (double-precision)" :default 0.0))
  (bind _elevation (`self.Clamp Elevation` `Axis Input`))
  (bind _output_get (set `local.Local Elevation` _elevation))
  (if (< _output_get 0.0)
    (`SceneComponent.K2_SetRelativeRotation` (`self.Pivot 1`) (`KismetMathLibrary.MakeRotator` 0.0 (`local.Local Elevation`)) false false)
    (`SceneComponent.K2_SetRelativeRotation` (`self.Pivot 2`) (`KismetMathLibrary.MakeRotator` 0.0) false false)
    (else
      (`SceneComponent.K2_SetRelativeRotation` (`self.Pivot 2`) (`KismetMathLibrary.MakeRotator` 0.0 (`local.Local Elevation`)) false false)
      (`SceneComponent.K2_SetRelativeRotation` (`self.Pivot 1`) (`KismetMathLibrary.MakeRotator` 0.0) false false)))
  (return (`local.Local Elevation`)))

(fn `UserConstructionScript`
  (`parent.UserConstructionScript`)
  (`SceneComponent.K2_SetRelativeLocation` (`self.Zoom Camera`) (150.0 0.0 35.0) false false))