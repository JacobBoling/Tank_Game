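; BP_Artillery is an artillery turret for a tank, built on a parent turret class.
; Its construction script adds an AC Path Weapon component configured with limited ammo, a firing delay, projectile damage and speed, muzzle particles and camera shake.
; On BeginPlay it offsets the tank's camera.
; Fire triggers the weapon and, only when a shot succeeds, plays a timeline that drives the cannon's recoil.
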(event `self.ReceiveBeginPlay`
  (`parent.ReceiveBeginPlay`)
  (`/Game/Parents/BP_Tank.Move Camera` (`self.Tank`) (0.0 -50.0 0.0)))

(event `self.Fire`
  (bind _return (`/Game/Magnus/Tank/Components/Actor_Components/AC_Weapon.Fire` (`self.Weapon`)))
  (if _return
    (bind (_direction _recoil) (`Timeline|Recoil Timeline` :!via `PlayFromStart`)
      (:`Update`
        (`/Game/Magnus/Tank/Components/Actor_Components/AC_Weapon.Recoil Cannon` (`self.Weapon`) _recoil)))))

(fn `UserConstructionScript`
  (`parent.UserConstructionScript`)
  (bind _returnvalue (`AddComponent|NODE_AddAC_Path_Weapon-0` :`Max Ammo` 25 :`Firing Delay` 3.0 :`Particles` "/Game/Magnus/Tank/Components/Particles/FXS_Firing_Particles.FXS_Firing_Particles" :`Casing` null :`Cam Shake` "/Game/Magnus/Tank/Components/Cam_Shake/AC_Cam_Shake.AC_Cam_Shake_C" :`Turret` self :`Impact Damage` 50.0 :`Muzzle Velocity` 12000.0 :`Projectile Radius` 20.0))
  (bind _output_get (set `self.Path Weapon` _returnvalue))
  (set `self.Weapon` _output_get))