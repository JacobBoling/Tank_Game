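; BP_Tank_Destroyer is the tank destroyer turret, firing a slow, limited-ammo cannon with its own projectile class.
; The construction script sets Pivot1 as the rotator and adds an ammo weapon component with firing particles and camera shake.
; Fire triggers the weapon and, on a successful shot, plays a timeline that drives cannon recoil.
; BeginPlay offsets the owning tank's camera along negative X.
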(event `self.ReceiveBeginPlay`
  (`parent.ReceiveBeginPlay`)
  (`/Game/Parents/BP_Tank.Move Camera` (`self.Tank`) (-310.0 0.0 0.0)))

(event `self.Fire`
  (bind _return (`/Game/Magnus/Tank/Components/Actor_Components/AC_Weapon.Fire` (`self.Weapon`)))
  (if _return
    (bind (_direction _recoil) (`Timeline|Recoil Timeline` :!via `PlayFromStart`)
      (:`Update`
        (`/Game/Magnus/Tank/Components/Actor_Components/AC_Weapon.Recoil Cannon` (`self.Weapon`) _recoil)))))

(fn `UserConstructionScript`
  (`parent.UserConstructionScript`)
  (set `self.Rotator` (`self.Pivot 1`))
  (bind _returnvalue (`AddComponent|NODE_AddAC_Ammo_Weapon-0` :`Max Ammo` 25 :`Firing Delay` 2.0 :`Particles` "/Game/Magnus/Tank/Components/Particles/FXS_Firing_Particles.FXS_Firing_Particles" :`Casing` null :`Cam Shake` "/Game/Magnus/Tank/Components/Cam_Shake/AC_Cam_Shake.AC_Cam_Shake_C" :`Turret` self :`Projectile Class` "/Game/Magnus/Projectile/BP_Proj_Mag_TD.BP_Proj_Mag_TD_C"))
  (bind _output_get (set `self.Ammo Weapon` _returnvalue))
  (set `self.Weapon` _output_get))