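; Player controller for a tank game that handles the overview camera phase, spawning, pausing and killfeed updates.
; On begin play and after a match ends, it shows the overview menu and camera while a timer counts down to Spawn.
; Spawn restarts the player at a start point, then replaces that pawn with the tank and turret from the PlayerState loadout.
; Pause toggles a cached menu, cursor and pawn input without pausing the game.
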(event Custom|Generate%20Pawn
  (params (Location :type Transform))
  (Actor|DestroyActor (Variables|Default|GetPossessed%20Pawn))
  (bind _asbp_tank_player_state (Utilities|Casting|CastToBP_Tank_Player_State (Variables|GetPlayerState)))
  (bind _returnvalue (Game|SpawnActorfromClass (.tank (Variables|/Game/Menus/BP_Tank_Player_State.BP_Tank_Player_State_C|GetLoadout _asbp_tank_player_state)) Location "Undefined" "MultiplyWithRoot" 0 (.turret (Variables|/Game/Menus/BP_Tank_Player_State.BP_Tank_Player_State_C|GetLoadout _asbp_tank_player_state)) 0))
  (Pawn|Possess _returnvalue))

(event Custom|Enter%20Overview
  (params (Timer%20Function :type String) (Time :type Float%20%28single-precision%29))
  (bind _returnvalue (Utilities|Time|SetTimerbyFunctionName 0 Timer%20Function Time))
  (bind _returnvalue_2 (UserInterface|CreateWidget "/Game/Menus/WBP_Overview_Menu.WBP_Overview_Menu_C" self _returnvalue))
  (UserInterface|Viewport|AddtoViewport _returnvalue_2 0)
  (Variables|Default|SetbShowMouseCursor true)
  (Game|Player|SetViewTargetwithBlend (Variables|Default|GetOverview%20Cam) 0.1 "VTBlend_Linear" 0.0 false))

(event Custom|Pause%20Game
  (bind _returnvalue (Pawn|GetControlledPawn))
  (bind _self self)
  (Utilities|IsValid (Variables|Default|GetPause%20Menu)
    (:Is%20Valid
      (if (Variables|Default|GetPaused)
        (Widget|RemovefromParent (Variables|Default|GetPause%20Menu))
        (Variables|Default|SetPaused false)
        (Variables|Default|SetbShowMouseCursor false)
        (Input|EnableInput _returnvalue _self)
        (else
          (UserInterface|Viewport|AddtoViewport (stale _output_get) 0 :!label _label)
          (Variables|Default|SetPaused true)
          (Variables|Default|SetbShowMouseCursor true)
          (Input|DisableInput _returnvalue _self))))
    (:Is%20Not%20Valid
      (bind _returnvalue_2 (UserInterface|CreateWidget "/Game/Menus/WBP_Pause_Menu.WBP_Pause_Menu_C" self))
      (bind _output_get (Variables|Default|SetPause%20Menu _returnvalue_2))
      (goto _label))))

(event Custom|Spawn
  (bind _returnvalue (Game|GetGameMode))
  (bind _self self)
  (Class|GameModeBase|RestartPlayeratPlayerStart _returnvalue _self (Class|GameModeBase|FindPlayerStart _returnvalue _self))
  (CallFunction|GeneratePawn (Transformation|GetActorTransform (Variables|Default|GetPossessed%20Pawn)))
  (Variables|Default|SetbShowMouseCursor false))

(event Custom|Notify%20Killfeed
  (params (Kill%20Event :type F%20Kill%20Event%20Structure))
  (bind _asbp_tank_hud (Utilities|Casting|CastToBP_Tank_HUD (HUD|GetHUD)))
  (Default|AddKill (Variables|/Game/Magnus/BP_Tank_HUD.BP_Tank_HUD_C|GetKillfeed _asbp_tank_hud) Kill%20Event))

(event Custom|End%20Game
  (if (Variables|Default|GetPaused)
    (CallFunction|PauseGame))
  (Input|DisableInput (Pawn|GetControlledPawn) self)
  (Utilities|FlowControl|Delay 5.0)
  (CallFunction|EnterOverview "Spawn" 3e+01))

(event Input|EnhancedActionEvents|EnhancedInputActionIA_Pause
  (params (ActionValue :type Boolean) (ElapsedSeconds :type Float%20%28double-precision%29) (TriggeredSeconds :type Float%20%28double-precision%29) (InputAction :type Input%20Action%20Object%20Reference :default "/Game/Inputs/IA_Pause.IA_Pause"))
  (:Triggered
    (CallFunction|PauseGame)))

(event EventBeginPlay
  (Utilities|FlowControl|DelayUntilNextTick)
  (bind _returnvalue (Actor|GetActorOfClass "/Script/Engine.CameraActor"))
  (Variables|Default|SetOverview%20Cam _returnvalue)
  (CallFunction|EnterOverview "Spawn" 15.0))

(event EventPossess
  (params (PossessedPawn :type Pawn%20Object%20Reference))
  (Variables|Default|SetPossessed%20Pawn PossessedPawn))

(event Input|KeyboardEvents|DebugKeyT
  (params (Key :type Key%20Structure :default "None") (ActionValue :type Input%20Action%20Value%20Structure)))

(fn ConstructionScript)