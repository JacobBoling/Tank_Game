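; AC_Path_Weapon is a tank weapon component that predicts the cannon's projectile path for the HUD.
; BeginPlay caches BP_Tank_HUD through the ammo widget's owning player.
; Every Tick, TraceLine runs a projectile-path prediction from the Muzzle socket using muzzle velocity, ignoring the turret, and writes the positions and final trace destination into the HUD's Points.
; The BP_Hit_Indicator endpoint logic is disconnected and never runs.
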(event `self.ReceiveBeginPlay`
  (`parent.ReceiveBeginPlay`)
  (bind _asbp_tank_hud (cast `/Game/Magnus/BP_Tank_HUD` (`PlayerController.GetHUD` (`Widget.GetOwningPlayer` (`self.HUD Ammo Ref`)))))
  (set `self.HUD` _asbp_tank_hud))

(event `self.ReceiveTick`
  (params (DeltaSeconds :type "Float (single-precision)"))
  (`self.Trace Line`))

(event `Trace Line`
  (bind _cannon (`self.Cannon`))
  (bind (_outhit _outpathpositions _outlasttracedestination) (`GameplayStatics.Blueprint_PredictProjectilePath_ByTraceChannel` (`SceneComponent.GetSocketLocation` _cannon "Muzzle") (* (`SceneComponent.GetForwardVector` _cannon) (`self.Muzzle Velocity`)) true (`self.Projectile Radius`) "ECC_GameTraceChannel1" false (`|MakeArray` (`self.Turret`) :!type "Actor Object Reference")))
  (bind _output_get (set `/Game/Magnus/BP_Tank_HUD.Points` _outpathpositions (`self.HUD`)))
  (`KismetArrayLibrary.Array_Add` _output_get _outlasttracedestination))