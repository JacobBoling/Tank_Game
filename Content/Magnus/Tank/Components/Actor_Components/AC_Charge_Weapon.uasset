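; Actor component for a tank charge weapon that fires a hitscan shot from the turret cannon.
; Fire, when allowed, clears the firing flags, line-traces from the Muzzle socket out to Range and sends the hit actor a fixed damage message crediting the tank.
; No charge logic appears here; Tick defers to the parent, and the reload-percentage and reticle-progress logic is left unused.
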(event `self.ReceiveTick`
  (params (DeltaSeconds :type "Float (single-precision)"))
  (`parent.ReceiveTick` DeltaSeconds))

(fn `Fire`
  (returns (Return :type Boolean))
  (bind (_returnvalue_location _returnvalue_rotation) (`KismetMathLibrary.BreakTransform` (`SceneComponent.GetSocketTransform` (`/Game/Parents/BP_Turret.Cannon` (`self.Turret`)) "Muzzle" "RTS_World")))
  (if (`self.Can Fire`)
    (set `self.Firing` false)
    (set `self.Can Fire` false)
    (bind _outhit (`KismetSystemLibrary.LineTraceSingle` _returnvalue_location (+ _returnvalue_location (* (`KismetMathLibrary.GetForwardVector` _returnvalue_rotation) (`self.Range`))) "TraceTypeQuery1"))
    (message `/Game/Magnus/Tank/Components/BI_Damageable.Modify Health` (`.HitActor` (`GameplayStatics.BreakHitResult` _outhit)) (`/Game/Parents/BP_TankPart.Tank` (`self.Turret`)) 60.0 "NewEnumerator0")
    (return true)
    (else
      (return false))))